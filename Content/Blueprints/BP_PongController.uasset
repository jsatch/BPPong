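; BP_PongController is the Pong controller that turns player movement input into sideways motion of the paddle.
; On the Enhanced Input IA_Move action, it casts player 0's pawn to BP_Paddle and shifts that paddle's Box component along world X by speed, input value and delta time.
; The new X is clamped to fixed symmetric limits while Y and Z are preserved, and a failed cast prints an error.
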(event Input|EnhancedActionEvents|EnhancedInputActionIA_Move
  (params (ActionValue :type Float%20%28double-precision%29) (ElapsedSeconds :type Float%20%28double-precision%29) (TriggeredSeconds :type Float%20%28double-precision%29) (InputAction :type Input%20Action%20Object%20Reference :default "/Game/InputSystem/IA_Move.IA_Move"))
  ;[1 1 1] Handling Movement
  (bind _asbp_paddle (Utilities|Casting|CastToBP_Paddle (Game|Player|GetPlayerPawn 0))
    (:then
      (Transformation|SetWorldLocation (Variables|/Game/Blueprints/BP_Paddle.BP_Paddle_C|GetBox _asbp_paddle) (Math|Vector|MakeVector (Math|Float|Clamp(Float) (+ (.x (Transformation|GetWorldLocation (Variables|/Game/Blueprints/BP_Paddle.BP_Paddle_C|GetBox _asbp_paddle))) (* (Variables|/Game/Blueprints/BP_Paddle.BP_Paddle_C|GetSpeed _asbp_paddle) ActionValue (Utilities|Time|GetWorldDeltaSeconds))) -3e+02 3e+02) (.y (Transformation|GetWorldLocation (Variables|/Game/Blueprints/BP_Paddle.BP_Paddle_C|GetBox _asbp_paddle))) (.z (Transformation|GetWorldLocation (Variables|/Game/Blueprints/BP_Paddle.BP_Paddle_C|GetBox _asbp_paddle)))) false false))
    (:CastFailed
      (Development|PrintString "ERROR Casting"))))

(fn ConstructionScript)