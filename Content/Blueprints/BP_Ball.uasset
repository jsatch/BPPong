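; BP_Ball is the ball for a paddle-and-wall game, moving each tick along a Velocity direction through FloatingPawnMovement input.
; Sphere overlaps redirect it: walls flip X, while paddles flip Y and randomize X.
; Overlapping a goal zone calls the Goal event, which spawns a fresh ball at a fixed location, then destroys this one.
; A debug line trace of the velocity is present but never executes.
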(event OnComponentBeginOverlap(SphereCollider)
  (params (OverlappedComponent :type Primitive%20Component%20Object%20Reference) (OtherActor :type Actor%20Object%20Reference) (OtherComp :type Primitive%20Component%20Object%20Reference) (OtherBodyIndex :type Integer) (bFromSweep :type Boolean) (SweepResult :type Hit%20Result%20Structure%20%28by%20ref%29))
  (Utilities|Casting|CastToBP_Wall OtherActor
    (:then
      (Variables|Default|SetVelocity (Math|Vector|MakeVector (* (.x (Variables|Default|GetVelocity)) -1.0) (.y (Variables|Default|GetVelocity)) (.z (Variables|Default|GetVelocity)))))
    (:CastFailed
      (Utilities|Casting|CastToBP_Paddle OtherActor
        (:then
          (Variables|Default|SetVelocity (Math|Vector|MakeVector (Math|Random|RandomFloatinRange -1.0 1.0) (* (.y (Variables|Default|GetVelocity)) -1.0) (.z (Variables|Default|GetVelocity)))))
        (:CastFailed
          (Utilities|Casting|CastToBP_GoalZone OtherActor)
          ;[1 1 1] Goal
          (CallFunction|Goal)
          (Actor|DestroyActor))))))

(event Custom|Goal
  (Game|SpawnActorfromClass "BP_Ball_C" (Math|Transform|MakeTransform "0.000000,40.000000,10.000000") "Undefined" "MultiplyWithRoot" 0 0))

(event EventTick
  (params (DeltaSeconds :type Float%20%28single-precision%29))
  (Class|PawnMovementComponent|AddInputVector (Variables|Default|GetFloatingPawnMovement) (Math|Vector|Normalize (Variables|Default|GetVelocity)) false))

(event EventBeginPlay
  (Variables|Default|SetVelocity "0.000000,-1.000000,0.000000"))

(fn ConstructionScript)