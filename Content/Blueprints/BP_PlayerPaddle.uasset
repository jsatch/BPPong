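; BP_PlayerPaddle is a player-controlled paddle that sets up Enhanced Input but does not yet move.
; On BeginPlay it casts its controller to PlayerController and adds the IC_Gameplay mapping context to the local player's input subsystem.
; The IA_Move event is empty.
; An unconnected AddWorldOffset node holds the intended X-axis movement, scaled by input value, Speed and frame delta time.
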(event Input|EnhancedActionEvents|EnhancedInputActionIA_Move
  (params (ActionValue :type Float%20%28double-precision%29) (ElapsedSeconds :type Float%20%28double-precision%29) (TriggeredSeconds :type Float%20%28double-precision%29) (InputAction :type Input%20Action%20Object%20Reference :default "/Game/InputSystem/IA_Move.IA_Move")))

(event EventBeginPlay
  ;[1 1 1] Configure Mapping Context (New Input System)
  (bind _asplayer_controller (Utilities|Casting|CastToPlayerController (Pawn|GetController)))
  (Utilities|IsValid (PlayerController|LocalPlayerSubsystems|GetEnhancedInputLocalPlayerSubsystem _asplayer_controller)
    (:Is%20Valid
      (Input|AddMappingContext (PlayerController|LocalPlayerSubsystems|GetEnhancedInputLocalPlayerSubsystem _asplayer_controller) "/Game/InputSystem/IC_Gameplay.IC_Gameplay" 0 "(bIgnoreAllPressedKeysUntilRelease=True,bForceImmediately=False,bNotifyUserSettings=False)"))))

(fn ConstructionScript)