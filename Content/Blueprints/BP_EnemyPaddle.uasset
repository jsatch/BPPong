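; BP_EnemyPaddle is the computer-controlled paddle, which slides along the X axis in response to the ball.
; Every Tick it looks up BP_Ball and steps by Speed and delta time in the direction of the sign of the ball's world X.
; It compares against world zero rather than its own position, and clamps X to a fixed symmetric range while keeping Y and Z.
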(event EventBeginPlay)

(event EventTick
  (params (DeltaSeconds :type Float%20%28single-precision%29))
  (bind _returnvalue (Transformation|GetActorLocation))
  (bind _returnvalue_2 (Actor|GetActorOfClass "/Game/Blueprints/BP_Ball.BP_Ball_C"))
  (Transformation|SetActorLocation (Math|Vector|MakeVector (Math|Float|Clamp(Float) (+ (* (Math|Float|Sign(Float) (.x (Transformation|GetActorLocation _returnvalue_2))) (Variables|Default|GetSpeed) (Utilities|Time|GetWorldDeltaSeconds)) (.x _returnvalue)) -3e+02 3e+02) (.y _returnvalue) (.z _returnvalue)) false false))

(fn ConstructionScript
  (|CallParentFunction))